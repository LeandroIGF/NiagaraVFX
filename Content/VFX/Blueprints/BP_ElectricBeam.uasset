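; BP_ElectricBeam is an actor that drives a Niagara electric beam aimed at a target actor, ActorBeamEnd.
; Each Tick, while the target is valid, it runs a Visibility line trace from the Niagara component for a fixed length in the target's direction.
; The blocking-hit result sets the Collision parameter, and SetBeamEndLocation writes the impact point or trace end to BeamEnd in actor-local space.
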(event `self.ReceiveTick`
  (params (DeltaSeconds :type "Float (single-precision)"))
  (bind _returnvalue (`SceneComponent.K2_GetComponentLocation` (`self.Niagara`)))
  (`/Engine/EditorBlueprintResources/StandardMacros.IsValid` (`self.ActorBeamEnd`)
    (:`Is Valid`
      (set `self.End BeamTrace` (+ _returnvalue (* (`KismetMathLibrary.Normal` (- (`self.K2_GetActorLocation` (`self.ActorBeamEnd`)) (`self.K2_GetActorLocation`))) 600.0)))
      (bind _outhit (`KismetSystemLibrary.LineTraceSingle` _returnvalue (`self.End BeamTrace`) "TraceTypeQuery1"))
      (bind (_bblockinghit _binitialoverlap _time _distance _location _impactpoint) (`GameplayStatics.BreakHitResult` _outhit))
      (`NiagaraComponent.SetVariableBool` (`self.Niagara`) "Collision" _bblockinghit)
      (if _bblockinghit
        (`self.SetBeamEndLocation` _impactpoint)
        (else
          (`self.SetBeamEndLocation` (`self.End BeamTrace`)))))))

(fn `SetBeamEndLocation`
  (params (EndBeamLocation :type "Vector Structure"))
  (`NiagaraComponent.SetVariableVec3` (`self.Niagara`) "BeamEnd" (`KismetMathLibrary.InverseTransformLocation` (`self.GetTransform`) EndBeamLocation)))

(fn `UserConstructionScript`)