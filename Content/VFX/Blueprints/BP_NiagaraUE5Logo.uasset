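; Blueprint that displays a Niagara UE5 logo effect with two animated colors.
; The construction script applies the Color1 and Color2 variables to the effect's matching color parameters.
; On BeginPlay, the TimelineColor timeline starts, overriding both parameters on each update and restarting when finished to loop the color animation.
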(event `self.ReceiveBeginPlay`
  (`TimelineComponent.PlayFromStart` (`self.TimelineColor`)))

(fn `UserConstructionScript`
  (`FXSystemComponent.SetColorParameter` (`self.NiagaraUE5Logo`) "Color1" (`self.Color1`))
  (`FXSystemComponent.SetColorParameter` (`self.NiagaraUE5Logo`) "Color2" (`self.Color2`)))